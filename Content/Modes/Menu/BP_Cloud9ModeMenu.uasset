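; BP_Cloud9ModeMenu is the menu mode Blueprint that plays the main menu music and a dust2 background sound.
; On BeginPlay, PlayBackgroundSounds spawns both as 2D sounds, with volumes read from a fetched settings object.
; Playback-percent callbacks store each track's elapsed time, so calling PlayBackgroundSounds again destroys the old components and resumes from the saved positions.
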(event Custom|PlayBackgroundSounds
  (Utilities|IsValid (Variables|Default|GetMainmenuSound)
    (:Is%20Valid
      (Components|DestroyComponent (Variables|Default|GetMainmenuSound))
      (Utilities|IsValid (Variables|Default|GetBackgroundSound)
        (:Is%20Valid
          (Components|DestroyComponent (Variables|Default|GetBackgroundSound)))
        (:Is%20Not%20Valid
          _)))
    (:Is%20Not%20Valid
      _))
  (bind _returnvalue (Class|Cloud9DeveloperSettings|Get))
  (bind _returnvalue_2 (Audio|SpawnSound2D "/Game/HUD/Sounds/mainmenu.mainmenu" (Variables|/Script/Cloud9.Cloud9DeveloperSettings|GetMainMenuMusicVolume _returnvalue) 1.0 0.0 0 false false))
  (bind _output_get (Variables|Default|SetMainmenuSound _returnvalue_2))
  (EventDispatchers|BindEventtoOnAudioPlaybackPercent _output_get (delegate Custom|OnMainMenuSoundPlayback))
  (Audio|Components|Audio|Play (Variables|Default|GetMainmenuSound) (Variables|Default|GetElapsedTimeMainmenu))
  (bind _returnvalue_3 (Audio|SpawnSound2D "/Game/HUD/Sounds/bg_dust2_01.bg_dust2_01" (* (Variables|/Script/Cloud9.Cloud9DeveloperSettings|GetVolume _returnvalue) 16.0) 1.0 0.0 0 false false))
  (bind _output_get_2 (Variables|Default|SetBackgroundSound _returnvalue_3))
  (EventDispatchers|BindEventtoOnAudioPlaybackPercent _output_get_2 (delegate Custom|OnBackgroundSoundPlayback))
  (Audio|Components|Audio|Play (Variables|Default|GetBackgroundSound) (Variables|Default|GetElapsedTimeBackground)))

(event Custom|OnMainMenuSoundPlayback
  (params (PlayingSoundWave :type Sound%20Wave%20Object%20Reference) (PlaybackPercent :type Float%20%28single-precision%29))
  (Variables|Default|SetElapsedTimeMainmenu (* (Variables|/Script/Engine.SoundBase|GetDuration PlayingSoundWave) PlaybackPercent)))

(event Custom|OnBackgroundSoundPlayback
  (params (PlayingSoundWave :type Sound%20Wave%20Object%20Reference) (PlaybackPercent :type Float%20%28single-precision%29))
  (Variables|Default|SetElapsedTimeBackground (* (Variables|/Script/Engine.SoundBase|GetDuration PlayingSoundWave) PlaybackPercent)))

(event EventBeginPlay
  (CallFunction|PlayBackgroundSounds))

(fn ConstructionScript)