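; BP_Cloud9Console provides debug command events for loading maps, selecting weapons and testing camera shake.
; Map shows a loading widget, then async-loads and opens the named level under /Game/Maps.
; Shake prints the player's location and plays a test camera shake for a clamped duration.
; SelectWeapon only fetches the game mode; its inventory selection call is disconnected and never runs.
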(event Custom|Map
  (params (Name :type String))
  (bind _returnvalue (Utilities|String|Append "/Game/Maps/" Name))
  (bind _returnvalue_2 (Utilities|String|StringToName _returnvalue))
  (Development|PrintString (Utilities|String|Append "Loading: " Name) true true "(R=1.000000,G=0.000000,B=0.000000,A=1.000000)")
  (bind _returnvalue_3 (UserInterface|CreateWidget "/Game/Blueprints/Widgets/MapLoadWidget.MapLoadWidget_C"))
  (Variables|/Game/Blueprints/Widgets/MapLoadWidget.MapLoadWidget_C|SetMap _returnvalue_3 Name)
  (UserInterface|Viewport|AddtoViewport _returnvalue_3 0)
  (Utilities|FlowControl|Delay 0.2)
  (Utilities|AsyncLoadAsset (Class|KismetSystemLibrary|GetSoftObjectReferencefromPrimaryAssetId (Utilities|Struct|MakePrimaryAssetId "Map" _returnvalue_2))
    (:Completed
      (Game|OpenLevel(byName) _returnvalue_2))))

(event Custom|Shake
  (params (Duration :type Float%20%28single-precision%29))
  (bind _returnvalue (Game|GetPlayerCameraManager 0))
  (Development|PrintString (Utilities|String|ToString(Vector) (Transformation|GetActorLocation (Game|GetPlayerCharacter 0))))
  (bind _returnvalue_2 (Class|MatineeCameraShake|StartMatineeCameraShake _returnvalue "/Game/Blueprints/Test/BP_CameraShakeTest.BP_CameraShakeTest_C" 1.0 "CameraLocal" "0, 0, 0"))
  (Utilities|FlowControl|Delay (Math|Float|Clamp(Float) Duration 1.0 3e+01))
  (CameraShakes|StopCameraShake _returnvalue _returnvalue_2 true))

(event Custom|SelectWeapon
  (params (Weapon :type Integer))
  (bind _returnvalue (Class|Cloud9ToolsLibrary|GetGameMode)))