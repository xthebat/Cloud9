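; Weapon pickup spawner, marked deprecated by name, that displays a configured weapon and grants it to the Cloud9 character that walks into it.
; On BeginPlay it applies the config to a weapon initializer child actor, optionally starts a colored glow effect and randomizes initial yaw, then binds a child trigger box's overlap.
; Tick spins the displayed weapon, and overlap force-adds and selects the weapon in the character's inventory.
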(event Custom|OnReplaceWeaponEntry
  (params (OverlappedActor :type Actor%20Object%20Reference) (OtherActor :type Actor%20Object%20Reference))
  (bind _asbp_cloud_9character (Utilities|Casting|CastToBP_Cloud9Character OtherActor))
  (Class|Cloud9Inventory|AddWeapon (Variables|/Script/Cloud9.Cloud9Character|GetInventory _asbp_cloud_9character) (Variables|Weapon|GetConfig) true true))

(event EventBeginPlay
  (bind _weaponinitializer (Variables|Default|GetWeaponInitializer))
  (bind _glowingcomponent (Variables|Default|GetGlowingComponent))
  (bind _childactor (Variables|/Script/Engine.ChildActorComponent|GetChildActor _weaponinitializer))
  (bind _returnvalue (Transformation|GetActorRotation _childactor))
  (if (Variables|Default|GetGlowingEnabled)
    (Components|Activation|Activate _glowingcomponent true)
    (Niagara|SetNiagaraVariable(LinearColor) _glowingcomponent "Color" (Variables|Default|GetGlowingColor))
    (Niagara|SetNiagaraVariable(Float) _glowingcomponent "Rate" (Variables|Default|GetGlowingSpeed)))
  (Class|WeaponInitializerComponent|SetWeaponConfig (Variables|Default|GetWeaponInitializer) (Variables|Weapon|GetConfig))
  (Utilities|IsValid (Variables|/Script/Engine.ChildActorComponent|GetChildActor (Variables|Default|GetWeaponInitializer))
    (:Is%20Valid
      (bind _astrigger_box (Utilities|Casting|CastToTriggerBox (Variables|/Script/Engine.ChildActorComponent|GetChildActor (Variables|Default|GetTriggerZone))))
      (Collision|BindEventtoOnActorBeginOverlap _astrigger_box (delegate Custom|OnReplaceWeaponEntry))
      (if (Variables|Default|GetRandomInitialRotation)
        (Transformation|SetActorRotation _childactor (Math|Rotator|MakeRotator (.roll _returnvalue) (.pitch _returnvalue) (* (Math|Random|RandomFloat) 3.6e+02)))))))

(event EventTick
  (params (DeltaSeconds :type Float%20%28single-precision%29))
  (bind _weaponinitializer (Variables|Default|GetWeaponInitializer))
  (bind _childactor (Variables|/Script/Engine.ChildActorComponent|GetChildActor _weaponinitializer))
  (bind _returnvalue (Transformation|GetActorRotation _childactor))
  (Utilities|IsValid _childactor
    (:Is%20Valid
      (Transformation|SetActorRotation _childactor (Math|Rotator|MakeRotator (.roll _returnvalue) (.pitch _returnvalue) (+ (* (Variables|Default|GetRotationSpeed) DeltaSeconds) (.yaw _returnvalue)))))))

(fn ConstructionScript)