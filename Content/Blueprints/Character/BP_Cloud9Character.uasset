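; Player character Blueprint for Cloud9 with helper functions for firing the selected inventory weapon.
; PlayWeaponVFX plays a stance- and weapon-type montage and sound, and activates muzzle flash for firearms.
; AddImpulseToObject traces from the muzzle to the cursor hit point to push the struck component, gated by CanAddImpulse, whose physics check is unwired.
; The EventGraph chain joining these with a cooldown has no trigger, so it never runs.
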(event Input|MouseEvents|LeftMouseButton
  (params (Key :type Key%20Structure :default "None")))

(fn ConstructionScript)