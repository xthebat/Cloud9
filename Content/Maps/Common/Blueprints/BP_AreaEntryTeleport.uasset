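; BP_AreaEntryTeleport is a level transition actor that sends the player to another map on entering its trigger.
; On BeginPlay it casts the TriggerZone child actor to a TriggerBox and binds to its begin-overlap event.
; When the overlapping actor is player character 0, it activates a particle system, waits briefly, then opens the referenced Level by object reference.
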(event Custom|OnTeleportEntry
  (params (OverlappedActor :type Actor%20Object%20Reference) (OtherActor :type Actor%20Object%20Reference))
  (if (== OtherActor (Game|GetPlayerCharacter 0))
    (Components|Activation|Activate (Variables|Default|GetParticleSystem) true)
    (Utilities|FlowControl|Delay 0.2)
    (Game|OpenLevel(byObjectReference) (Variables|Default|GetLevel))))

(event EventBeginPlay
  (bind _astrigger_box (Utilities|Casting|CastToTriggerBox (Variables|/Script/Engine.ChildActorComponent|GetChildActor (Variables|Default|GetTriggerZone))))
  (Collision|BindEventtoOnActorBeginOverlap _astrigger_box (delegate Custom|OnTeleportEntry)))

(fn ConstructionScript)