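; BP_Cloud9PracticeRangeBase is a shooting practice range that shows live session stats on a widget component.
; On BeginPlay it caches the BP_ShootingRangeStats widget and binds the target-destroyed event and the widget's reset button.
; Kill count updates on each destroyed target, while Tick refreshes kills per minute and elapsed time, blanking both when not started.
; Reset restarts shooting and refreshes the kill display with zero.
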(event Custom|OnResetPressedEvent
  (Class|Cloud9PracticeSpawner|RestartShooting)
  (CallFunction|OnTargetDestroyedEvent))

(event Custom|OnTargetDestroyedEvent
  (params (Count :type Integer))
  (bind _statswidget (Variables|Default|GetStatsWidget))
  (bind _killed (Variables|/Game/Environment/BP_ShootingRangeStats.BP_ShootingRangeStats_C|GetKilled _statswidget))
  (if (Variables|Default|GetbIsStarted)
    (Rendering|Components|TextRender|SetText _killed (Utilities|Text|ToText(Integer) Count false true 1 3))
    (else
      (Rendering|Components|TextRender|SetText _killed ""))))

(event EventBeginPlay
  (bind _asbp_shooting_range_stats (Utilities|Casting|CastToBP_ShootingRangeStats (UserInterface|GetUserWidgetObject (Variables|Default|GetWidgetComponent))))
  (Variables|Default|SetStatsWidget _asbp_shooting_range_stats)
  (EventDispatchers|AssignOnTargetDestroyed (delegate Custom|OnTargetDestroyedEvent))
  (EventDispatchers|AssignOnPressed (Variables|/Game/Environment/BP_ShootingRangeStats.BP_ShootingRangeStats_C|GetResetButton (Variables|Default|GetStatsWidget)) (delegate Custom|OnResetPressedEvent)))

(event EventTick
  (params (DeltaSeconds :type Float%20%28single-precision%29))
  (bind _statswidget (Variables|Default|GetStatsWidget))
  (bind _statswidget_2 (Variables|Default|GetStatsWidget))
  (bind _kpmvalue (Variables|/Game/Environment/BP_ShootingRangeStats.BP_ShootingRangeStats_C|GetKpmValue _statswidget))
  (bind _elapsedvalue (Variables|/Game/Environment/BP_ShootingRangeStats.BP_ShootingRangeStats_C|GetElapsedValue _statswidget_2))
  (if (Variables|Default|GetbIsStarted)
    (Rendering|Components|TextRender|SetText _kpmvalue (Utilities|Text|ToText(Integer) (Math|Float|Truncate (Class|Cloud9PracticeSpawner|GetKillPerMinute)) false true 1 3))
    (Rendering|Components|TextRender|SetText _elapsedvalue (Utilities|Text|ToText(Float) (Variables|Default|GetTimeElapsed) "HalfToEven" false true 1 3 0 1))
    (else
      (Rendering|Components|TextRender|SetText _kpmvalue "")
      (Rendering|Components|TextRender|SetText _elapsedvalue ""))))

(fn ConstructionScript)