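; Practice range bot spawner that provides BP_Cloud9CharacterBot targets; its only active logic is the SpawnTarget function.
; SpawnTarget always spawns a bot at the given location with the spawner's rotation and ownership.
; When a random Skins pick is valid, it applies a random skeletal mesh, raises the bot by its capsule half-height, sets a short destroy-after delay and returns it.
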(event EventBeginPlay
  (|CallParentFunction) ; This node is disabled and will not be called.\nDrag off pins to build functionality.
)

(event Collision|EventActorBeginOverlap
  (params (OtherActor :type Actor%20Object%20Reference)))

(event EventTick
  (params (DeltaSeconds :type Float%20%28single-precision%29))
  (|CallParentFunction DeltaSeconds) ; This node is disabled and will not be called.\nDrag off pins to build functionality.
)

(fn ConstructionScript
  (|CallParentFunction))

(fn SpawnTarget
  (params (Location :type Vector :default "0, 0, 0"))
  (bind _skins (Variables|Default|GetSkins))
  (bind _outitem (Utilities|Array|Random _skins))
  (bind _returnvalue (Game|SpawnActorfromClass "/Game/Characters/Blueprints/BP_Cloud9CharacterBot.BP_Cloud9CharacterBot_C" (Math|Transform|MakeTransform Location (Transformation|GetActorRotation) "1,1,1") "AlwaysSpawn" self 0))
  (Utilities|IsValid _outitem
    (:Is%20Valid
      (Class|SkinnedMeshComponent|SetSkeletalMesh (Variables|/Script/Engine.Character|GetMesh _returnvalue) _outitem true)
      (Transformation|AddActorLocalOffset _returnvalue (Math|Vector|MakeVector 0.0 0.0 (Components|Capsule|GetScaledCapsuleHalfHeight (Variables|/Script/Engine.Character|GetCapsuleComponent _returnvalue))) false true)
      (Class|Cloud9Character|SetDestroyAfter _returnvalue 1.0)
      (return _returnvalue))
    (:Is%20Not%20Valid
      (return 0))))