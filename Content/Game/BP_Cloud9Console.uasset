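; Cloud9 console Blueprint providing debug and gameplay commands for bots, map loading, weapon selection and camera shake.
; Bot commands spawn skinned bots or teleport a random one at the last crosshair location, raised by capsule half-height, and set sideways moving offsets on all AI controllers.
; Map validates names through the Asset Registry, then shows a loading widget and async-loads before opening the level.
; Shake plays a test shake for a clamped duration.
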(event Custom|Map
  (params (Name :type String) (Options :type String))
  (bind _output_get (Variables|Default|SetMapName Name))
  (Variables|Default|SetMapFound false)
  (Development|PrintString (Utilities|String|Append "Loading: " _output_get) true true "(R=1.000000,G=0.000000,B=0.000000,A=1.000000)")
  (bind _outassetdata (Class|AssetRegistry|GetAssetsbyPath (Class|AssetRegistryHelpers|GetAssetRegistry) "/Game/Maps" false false))
  (bind _array_element (Utilities|Array|ForEachLoopwithBreak _outassetdata :!label _label)
    (:LoopBody
      (if (Variables|Default|GetMapFound)
        (goto _label Break)
        (elif (and (Utilities|Enum|Equal(Enum) (Variables|Default|GetMapName) (.RightS (Utilities|String|Split (Class|AssetRegistryHelpers|GetFullName _array_element) "." "IgnoreCase" "FromEnd"))) (.ReturnValue (Utilities|String|Split (Class|AssetRegistryHelpers|GetFullName _array_element) "." "IgnoreCase" "FromEnd")))
          (Variables|Default|SetMapFound true))))
    (:Completed
      (if (Variables|Default|GetMapFound)
        (bind _returnvalue (UserInterface|CreateWidget "/Game/Widgets/MapLoadWidget.MapLoadWidget_C"))
        (Variables|/Game/Widgets/MapLoadWidget.MapLoadWidget_C|SetMap _returnvalue (Variables|Default|GetMapName))
        (UserInterface|Viewport|AddtoViewport _returnvalue 0)
        (Utilities|FlowControl|Delay 0.2)
        (Utilities|AsyncLoadAsset (Class|KismetSystemLibrary|GetSoftObjectReferencefromPrimaryAssetId (Utilities|Struct|MakePrimaryAssetId "Map" (Utilities|String|StringToName (Utilities|String|Append "/Game/Maps/" (Variables|Default|GetMapName)))))
          (:Completed
            (Game|OpenLevel(byName) (Utilities|String|StringToName (Utilities|String|Append "/Game/Maps/" (Variables|Default|GetMapName))) true Options)))
        (else
          (Development|PrintString "Invalid map name specified" true true "(R=1.000000,G=0.000000,B=0.000000,A=1.000000)"))))))

(event Custom|Shake
  (params (Duration :type Float%20%28single-precision%29))
  (bind _returnvalue (Game|GetPlayerCameraManager 0))
  (Development|PrintString (Utilities|String|ToString(Vector) (Transformation|GetActorLocation (Game|GetPlayerCharacter 0))))
  (bind _returnvalue_2 (Class|MatineeCameraShake|StartMatineeCameraShake _returnvalue "/Game/Test/BP_CameraShakeTest.BP_CameraShakeTest_C" 1.0 "CameraLocal" "0, 0, 0"))
  (Utilities|FlowControl|Delay (Math|Float|Clamp(Float) Duration 1.0 3e+01))
  (CameraShakes|StopCameraShake _returnvalue _returnvalue_2 true))

(event Custom|bot_add
  (params (Skin :type Skeletal%20Mesh%20Object%20Reference) (Rotation :type Float%20%28single-precision%29))
  (bind _ascloud_9player_controller (Utilities|Casting|CastToCloud9PlayerController (Game|GetPlayerController 0)))
  (Utilities|IsValid Skin
    (:Is%20Valid
      (Variables|Default|SetActualSkin Skin))
    (:Is%20Not%20Valid
      (Variables|Default|SetActualSkin "/Game/Characters/Sas/Mesh/ctm_sas_varianta.ctm_sas_varianta")))
  (if (Variables|/Script/Cloud9.Cloud9MouseController|GetbIsLastCrosshairLocationValid (Variables|/Script/Cloud9.Cloud9PlayerController|GetMouseController _ascloud_9player_controller))
    (bind _returnvalue (Game|SpawnActorfromClass "/Game/Characters/Blueprints/BP_Cloud9CharacterBot.BP_Cloud9CharacterBot_C" (Math|Transform|MakeTransform (Variables|/Script/Cloud9.Cloud9MouseController|GetLastCrosshairLocation (Variables|/Script/Cloud9.Cloud9PlayerController|GetMouseController _ascloud_9player_controller)) (Math|Rotator|MakeRotator 0.0 0.0 Rotation) "1,1,1") "AlwaysSpawn" 0 0))
    (Class|SkinnedMeshComponent|SetSkeletalMesh (Variables|/Script/Engine.Character|GetMesh _returnvalue) (Variables|Default|GetActualSkin) true)
    (Transformation|AddActorLocalOffset _returnvalue (Math|Vector|MakeVector 0.0 0.0 (Components|Capsule|GetScaledCapsuleHalfHeight (Variables|/Script/Engine.Character|GetCapsuleComponent _returnvalue))) false true)))

(event Custom|SelectWeapon
  (params (Weapon :type Byte))
  (bind _ascloud_9character (Utilities|Casting|CastToCloud9Character (Game|GetPlayerCharacter 0)))
  (Class|Cloud9InventoryComponent|SelectWeapon (Variables|/Script/Cloud9.Cloud9Character|GetInventoryComponent _ascloud_9character) (Utilities|Enum|ByteToEnumEWeaponSlot Weapon) false false))

(event Custom|bot_place
  (bind _outactors (Actor|GetAllActorsOfClass "/Game/Characters/Blueprints/BP_Cloud9CharacterBot.BP_Cloud9CharacterBot_C"))
  (Utilities|IsValid (.OutItem (Utilities|Array|Random _outactors))
    (:Is%20Valid
      (bind _ascloud_9player_controller (Utilities|Casting|CastToCloud9PlayerController (Game|GetPlayerController 0)))
      (if (Variables|/Script/Cloud9.Cloud9MouseController|GetbIsLastCrosshairLocationValid (Variables|/Script/Cloud9.Cloud9PlayerController|GetMouseController _ascloud_9player_controller))
        (Transformation|SetActorLocation (.OutItem (Utilities|Array|Random _outactors)) (+ (Math|Vector|MakeVector 0.0 0.0 (Components|Capsule|GetScaledCapsuleHalfHeight (Variables|/Script/Engine.Character|GetCapsuleComponent (.OutItem (Utilities|Array|Random _outactors))))) (Variables|/Script/Cloud9.Cloud9MouseController|GetLastCrosshairLocation (Variables|/Script/Cloud9.Cloud9PlayerController|GetMouseController _ascloud_9player_controller))) false true)))))

(event Custom|bot_move
  (params (Distance :type Float%20%28single-precision%29))
  (bind _outactors (Actor|GetAllActorsOfClass "/Script/Cloud9.Cloud9AIController"))
  (for _array_element _outactors
    (bind _ascloud_9character (Utilities|Casting|CastToCloud9Character (Pawn|GetControlledPawn _array_element)))
    (bind _ascloud_9aicontroller (Utilities|Casting|CastToCloud9AIController _array_element))
    (Class|Cloud9AIController|SetMovingOffset _ascloud_9aicontroller (* (Transformation|GetActorRightVector _ascloud_9character) Distance))))