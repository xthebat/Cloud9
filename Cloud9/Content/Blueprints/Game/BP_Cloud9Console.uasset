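; BP_Cloud9Console provides two console-style debug events, NetGraph and Shake.
; NetGraph converts its enable flag to an integer and passes it to the game mode's net graph setting.
; Shake prints the first player character's location, plays the BP_CameraShakeTest matinee shake on that player's camera manager, then stops it immediately after a delay of the clamped duration.
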(event Custom|NetGraph
  (params (Enable :type Boolean))
  (bind _returnvalue (Class|Cloud9ToolsLibrary|GetGameMode))
  (Class|Cloud9GameMode|SetNetGraph _returnvalue (Math|Conversions|ToInteger(Boolean) Enable)))

(event Custom|Shake
  (params (Duration :type Float%20%28single-precision%29))
  (bind _returnvalue (Game|GetPlayerCameraManager 0))
  (Development|PrintString (Utilities|String|ToString(Vector) (Transformation|GetActorLocation (Game|GetPlayerCharacter 0))))
  (bind _returnvalue_2 (Class|MatineeCameraShake|StartMatineeCameraShake _returnvalue "/Game/Blueprints/Test/BP_CameraShakeTest.BP_CameraShakeTest_C" 1.0 "CameraLocal" "0, 0, 0"))
  (Utilities|FlowControl|Delay (Math|Float|Clamp(Float) Duration 1.0 3e+01))
  (CameraShakes|StopCameraShake _returnvalue _returnvalue_2 true))